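; VR player character Blueprint that maps motion controller input to locomotion, jumping and shooting.
; Left-stick axes feed movement input along the camera's right and forward vectors, scaled by MovementSpeed, so movement follows head direction.
; Left grip press triggers a jump, and right trigger press calls SpawnProjectile.
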(event Input|ActionEvents|InputActionTriggerPressedRight
  (params (Key :type Key%20Structure :default "None"))
  (:Pressed
    (Class|VRCharacter|SpawnProjectile)))

(event Input|ActionEvents|InputActionGripPressedLeft
  (params (Key :type Key%20Structure :default "None"))
  (:Pressed
    (Character|Jump)))

(event Input|AxisEvents|InputAxisMovementAxisLeft_X
  (params (AxisValue :type Float%20%28single-precision%29))
  ;[1 1 1] Movement
  (Pawn|Input|AddMovementInput (Math|Vector|GetRightVector (Variables|Default|GetCamera)) (* AxisValue (Variables|Default|GetMovement%20Speed)) false))

(event Input|AxisEvents|InputAxisMovementAxisLeft_Y
  (params (AxisValue :type Float%20%28single-precision%29))
  ;[1 1 1] Movement
  (Pawn|Input|AddMovementInput (Math|Vector|GetForwardVector (Variables|Default|GetCamera)) (* AxisValue (Variables|Default|GetMovement%20Speed)) false))

(fn ConstructionScript)